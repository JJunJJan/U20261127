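; BP_Switch is an overlap-triggered switch that drives other objects: a spawner and three movers (box, square, stair).
; Any actor beginning overlap calls DoSpawn on Spawn, then sets IsPlay to true on MoveBox, MoveSquere and MoveStair.
; Ending overlap sets those IsPlay flags back to false, with no call to Spawn and no check for other actors still overlapping.
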(event `self.ReceiveActorBeginOverlap`
  (params (OtherActor :type "Actor Object Reference"))
  (`|ExecutionSequence`
    (:`then_0`
      (`/Game/MyAsset/BP_Spawn.DoSpawn` (`self.Spawn`)))
    (:`then_1`
      (set `/Game/MyAsset/BP_MoveBox.IsPlay` true (`self.MoveBox`)))
    (:`then_2`
      (set `/Game/MyAsset/BP_MoveSquere.IsPlay` true (`self.MoveSquere`)))
    (:`then_3`
      (set `/Game/MyAsset/BP_MoveStair.IsPlay` true (`self.MoveStair`)))))

(event `self.ReceiveActorEndOverlap`
  (params (OtherActor :type "Actor Object Reference"))
  (set `/Game/MyAsset/BP_MoveBox.IsPlay` false (`self.MoveBox`))
  (set `/Game/MyAsset/BP_MoveSquere.IsPlay` false (`self.MoveSquere`))
  (set `/Game/MyAsset/BP_MoveStair.IsPlay` false (`self.MoveStair`)))

(fn `UserConstructionScript`)