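; BP_MoveBox is a Blueprint that oscillates its Cube component up and down while IsPlay is true.
; Each Tick steps LocationX by a fixed amount, flipping the Direction flag when the value passes either limit around zero.
; Despite its name, LocationX drives the cube's relative Z location.
; The step ignores delta time, so speed depends on frame rate.
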(event `self.ReceiveTick`
  (params (DeltaSeconds :type "Float (single-precision)"))
  (if (`self.IsPlay`)
    (if (`self.Direction`)
      (if (<= (`self.LocationX`) 100.0)
        (set `self.LocationX` (+ (`self.LocationX`) 10.0) :!label _label)
        (else
          (set `self.Direction` false)
          (set `self.LocationX` (+ (`self.LocationX`) -10.0) :!label _label_2)))
      (elif (>= (`self.LocationX`) -100.0)
        (goto _label_2)
        (else
          (set `self.Direction` true)
          (goto _label))))
    (`SceneComponent.K2_SetRelativeLocation` (`self.Cube`) (`KismetMathLibrary.MakeVector` 0.0 0.0 (`self.LocationX`)) false false)))

(fn `UserConstructionScript`)