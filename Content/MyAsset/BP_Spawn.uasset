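; Spawner actor that fills its Box volume with BP_Ball actors when its DoSpawn event is called.
; A while loop spawns each ball at a random point inside the box and increments BallCount until it exceeds MaxCount, allowing one ball beyond that value from zero.
; A red on-screen debug message then reports that the maximum count is reached.
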(event `DoSpawn`
  (bind _maxcount (`self.MaxCount`))
  (bind _returnvalue (<= (`self.BallCount`) _maxcount))
  (if _returnvalue
    (while _returnvalue
      (`|SpawnActorFromClass` "/Game/MyAsset/BP_Ball.BP_Ball_C" (`KismetMathLibrary.MakeTransform` (`KismetMathLibrary.RandomPointInBoundingBox` (`self.K2_GetActorLocation`) (`BoxComponent.GetScaledBoxExtent` (`self.Box`)))) "Undefined" "MultiplyWithRoot" null null)
      (set `self.BallCount` (+ (`self.BallCount`) 1))))
  (`KismetSystemLibrary.PrintString` (`KismetStringLibrary.Concat_StrStr` "Ball Count is Max" (`KismetStringLibrary.Conv_IntToString` _maxcount)) true true (struct :`R` 1.0 :`B` 0.086481 :`A` 1.0) 10.0))

(fn `UserConstructionScript`)