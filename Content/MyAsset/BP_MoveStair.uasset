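; BP_MoveStair moves its Cube component along a looping stair-shaped path in the Y-Z plane while IsPlay is true.
; On Tick, a six-state Switch climbs two steps, then descends and slides back toward the start.
; Each state nudges LocationY or LocationZ by a fixed amount and sets the relative location, advancing at its threshold.
; Movement ignores delta time, so speed depends on frame rate.
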(event `self.ReceiveTick`
  (params (DeltaSeconds :type "Float (single-precision)"))
  (if (`self.IsPlay`)
    (switch `/Game/MyAsset/EN_MoveStair` (`self.Switch`)
      (:`NewEnumerator0`
        (if (<= (`self.LocationZ`) 100.0)
          (set `self.LocationZ` (+ (`self.LocationZ`) 10.0))
          (`SceneComponent.K2_SetRelativeLocation` (`self.Cube`) (`KismetMathLibrary.MakeVector` 0.0 (`self.LocationY`) (`self.LocationZ`)) false false :!label _label)
          (else
            (set `self.Switch` "NewEnumerator1"))))
      (:`NewEnumerator1`
        (if (<= (`self.LocationY`) 100.0)
          (set `self.LocationY` (+ (`self.LocationY`) 10.0))
          (goto _label)
          (else
            (set `self.Switch` "NewEnumerator2"))))
      (:`NewEnumerator2`
        (if (<= (`self.LocationZ`) 200.0)
          (set `self.LocationZ` (+ (`self.LocationZ`) 10.0))
          (goto _label)
          (else
            (set `self.Switch` "NewEnumerator3"))))
      (:`NewEnumerator3`
        (if (<= (`self.LocationY`) 200.0)
          (set `self.LocationY` (+ (`self.LocationY`) 10.0))
          (goto _label)
          (else
            (set `self.Switch` "NewEnumerator4"))))
      (:`NewEnumerator4`
        (if (>= (`self.LocationZ`) 0.0)
          (set `self.LocationZ` (+ (`self.LocationZ`) -10.0))
          (goto _label)
          (else
            (set `self.Switch` "NewEnumerator5"))))
      (:`NewEnumerator5`
        (if (>= (`self.LocationY`) 0.0)
          (set `self.LocationY` (+ (`self.LocationY`) -10.0))
          (goto _label)
          (else
            (set `self.Switch` "NewEnumerator0")))))))

(fn `UserConstructionScript`)