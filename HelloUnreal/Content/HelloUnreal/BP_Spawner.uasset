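; BP_Spawner is an actor that spawns BP_Ball actors in batches at random points inside its Box component.
; Each DoSpawn call loops to spawn five balls with the spawner's rotation, printing each index and a completion message.
; A running total is checked only before each batch, so it can pass the limit of 20 before further calls just print a maximum warning.
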(event `DoSpawn`
  (bind _count (`self.Count`))
  (if (<= (`self.AllCount`) 20)
    (while (< _count 5)
      (`KismetSystemLibrary.PrintString` (`KismetStringLibrary.Concat_StrStr` "index : " (`KismetStringLibrary.Conv_IntToString` _count)) true true (struct :`G` 0.66 :`B` 1.0 :`A` 1.0) 10.0)
      (`|SpawnActorFromClass` "/Game/HelloUnreal/BP_Ball.BP_Ball_C" (`KismetMathLibrary.MakeTransform` (`KismetMathLibrary.RandomPointInBoundingBox` (`self.K2_GetActorLocation`) (`BoxComponent.GetScaledBoxExtent` (`self.Box`))) (`self.K2_GetActorRotation`)) "Undefined" "MultiplyWithRoot" null null)
      (set `self.Count` (+ (`self.Count`) 1))
      (set `self.AllCount` (+ (`self.AllCount`) 1)))
    (set `self.Count` 0)
    (`KismetSystemLibrary.PrintString` "Complete" true true (struct :`G` 0.66 :`B` 1.0 :`A` 1.0) 10.0)
    (else
      (`KismetSystemLibrary.PrintString` "Ball count is Maximum" true true (struct :`R` 1.0 :`B` 0.154357 :`A` 1.0) 10.0))))

(fn `UserConstructionScript`)